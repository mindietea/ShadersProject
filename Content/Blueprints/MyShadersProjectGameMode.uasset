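; Game mode that starts enemy spawning and shows the player HUD when play begins.
; BeginPlay takes the first B_Enemy_Spawner in the level and sets a looping timer that calls its SpawnEnemy by name at the EnemiesPerSecond rate.
; It then creates Player_HUD, adds it to the viewport and stores it; the node handing the game mode to the HUD as GameManager is disconnected.
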(event EventBeginPlay
  (bind _outactors (Actor|GetAllActorsOfClass "/Game/Blueprints/B_Enemy_Spawner.B_Enemy_Spawner_C"))
  (bind _output_get (Variables|Default|SetSpawner (Utilities|Array|Get(acopy) _outactors)))
  (Utilities|Time|SetTimerbyFunctionName _output_get "SpawnEnemy" (/ 1.0 (Variables|Default|GetEnemies%20Per%20Second)) true)
  ;[1 1 1] Display UI
  (bind _returnvalue (UserInterface|CreateWidget "/Game/UI/Player_HUD.Player_HUD_C"))
  (UserInterface|Viewport|AddtoViewport _returnvalue 0)
  (Variables|Default|SetPlayer_HUD _returnvalue))

(event EventTick
  (params (DeltaSeconds :type Float%20%28single-precision%29)))

(fn ConstructionScript)