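; SlimeController is an AI controller for the B_Slime enemy.
; On possession it caches the slime pawn and runs the SlimeTree behavior tree.
; AI perception updates write whether the ThirdPersonCharacter is currently sensed into the CanSeePlayer blackboard key.
; Walk and Run events forward to the possessed slime's matching functions.
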(event OnTargetPerceptionUpdated(AIPerception)
  (params (Actor :type Actor%20Object%20Reference) (Stimulus :type AI%20Stimulus%20Structure))
  (Utilities|Casting|CastToThirdPersonCharacter Actor)
  (AI|Components|Blackboard|SetValueasBool (AI|GetBlackboard 0) (Utilities|Name|MakeLiteralName "CanSeePlayer") (.bSuccessfullySensed (Utilities|Struct|BreakAIStimulus Stimulus))))

(event Custom|Run
  (Default|Run (Variables|Default|GetSlime)))

(event Custom|Walk
  (Default|Walk (Variables|Default|GetSlime)))

(event EventOnPossess
  (params (PossessedPawn :type Pawn%20Object%20Reference))
  (bind _asb_slime (Utilities|Casting|CastToB_Slime PossessedPawn))
  (Variables|Default|SetSlime _asb_slime)
  (AI|RunBehaviorTree "/Game/Blueprints/AI/SlimeTree.SlimeTree")
  (Development|PrintString "Hello"))

(fn ConstructionScript)